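; Interactive door Blueprint that swings open and closed and shows an on-screen prompt when the player is near.
; InteractiveAction uses a FlipFlop to alternately play and reverse the OpenAndCloseDoor timeline, which lerps the DoorFrame's relative rotation through a half turn.
; A UI_DoorOpenMessage widget, created at BeginPlay, is added to or removed from the viewport as the player character enters or leaves OverlapBox.
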(event `self.InteractiveAction`
  (`/Engine/EditorBlueprintResources/StandardMacros.FlipFlop`
    (:`A`
      (bind (_direction _doorrotation) (`Timeline|OpenAndCloseDoor` :!label _label)
        (:`Update`
          (`SceneComponent.K2_SetRelativeRotation` (`self.DoorFrame`) (`KismetMathLibrary.RLerp` (struct) (struct :`Yaw` -180.0) _doorrotation) false false))))
    (:`B`
      (goto _label :!via `Reverse`))))

(event `self.ReceiveBeginPlay`
  (bind _returnvalue (`|CreateWidget` "/Game/HouseOfChangwon/Blueprints/UI_DoorOpenMessage.UI_DoorOpenMessage_C"))
  (set `self.InteractDoor` _returnvalue))

(event `self.OverlapBox.OnComponentBeginOverlap`
  (params (OverlappedComponent :type "PrimitiveComponent Object Reference") (OtherActor :type "Actor Object Reference") (OtherComp :type "PrimitiveComponent Object Reference") (OtherBodyIndex :type Integer) (bFromSweep :type Boolean) (SweepResult :type "HitResult Structure (by ref)"))
  (if (== OtherActor (`GameplayStatics.GetPlayerCharacter` 0))
    (`UserWidget.AddToViewport` (`self.InteractDoor`) 0)))

(event `self.OverlapBox.OnComponentEndOverlap`
  (params (OverlappedComponent :type "PrimitiveComponent Object Reference") (OtherActor :type "Actor Object Reference") (OtherComp :type "PrimitiveComponent Object Reference") (OtherBodyIndex :type Integer))
  (if (== (`GameplayStatics.GetPlayerCharacter` 0) OtherActor)
    (`Widget.RemoveFromParent` (`self.InteractDoor`))))

(fn `UserConstructionScript`)