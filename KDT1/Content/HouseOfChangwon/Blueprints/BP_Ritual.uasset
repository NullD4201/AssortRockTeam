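; BP_Ritual is a ritual object that spins in place and can be picked up by the player, which destroys it.
; It creates a UI_GetRitual widget at BeginPlay, then shows or removes it as the player character enters or leaves its Capsule.
; The InteractRitual event destroys the actor only while that overlap flag is set.
; The spin is a fixed rotation step each Tick, so its speed depends on frame rate.
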(event `self.ReceiveBeginPlay`
  (bind _returnvalue (`|CreateWidget` "/Game/HouseOfChangwon/Blueprints/UI_GetRitual.UI_GetRitual_C"))
  (set `self.UI Ritual` _returnvalue))

(event `self.ReceiveTick`
  (params (DeltaSeconds :type "Float (single-precision)"))
  (`self.K2_AddActorLocalRotation` (struct :`Yaw` 0.5)))

(event `/Game/HouseOfChangwon/Blueprints/BPI_Ritual.InteractRitual`
  (if (`self.IsPlayerOverlap`)
    (`self.K2_DestroyActor`)))

(event `self.Capsule.OnComponentBeginOverlap`
  (params (OverlappedComponent :type "PrimitiveComponent Object Reference") (OtherActor :type "Actor Object Reference") (OtherComp :type "PrimitiveComponent Object Reference") (OtherBodyIndex :type Integer) (bFromSweep :type Boolean) (SweepResult :type "HitResult Structure (by ref)"))
  (if (== OtherActor (`GameplayStatics.GetPlayerCharacter` 0))
    (set `self.IsPlayerOverlap` true)
    (`UserWidget.AddToViewport` (`self.UI Ritual`) 0)))

(event `self.Capsule.OnComponentEndOverlap`
  (params (OverlappedComponent :type "PrimitiveComponent Object Reference") (OtherActor :type "Actor Object Reference") (OtherComp :type "PrimitiveComponent Object Reference") (OtherBodyIndex :type Integer))
  (if (== (`GameplayStatics.GetPlayerCharacter` 0) OtherActor)
    (set `self.IsPlayerOverlap` false)
    (`Widget.RemoveFromParent` (`self.UI Ritual`))))

(fn `UserConstructionScript`)