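; An interactive door that swings open and closed, with on-screen open and close prompts.
; InteractiveAction alternates through a FlipFlop, setting DoorOpen and playing or reversing a timeline that lerps DoorFrame's rotation.
; BeginPlay creates both prompt widgets, and OverlapBox shows or removes the one matching DoorOpen as the player character enters or leaves.
; The timeline's update also swaps the prompts on every tick while the door moves.
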(event `self.InteractiveAction`
  (bind _interactdooropen (`self.InteractDoorOpen`))
  (bind _interactdoorclose (`self.InteractDoorClose`))
  (`/Engine/EditorBlueprintResources/StandardMacros.FlipFlop`
    (:`A`
      (set `self.DoorOpen` true)
      (bind (_direction _doorrotation) (`Timeline|OpenAndCloseDoor` :!label _label)
        (:`Update`
          (`SceneComponent.K2_SetRelativeRotation` (`self.DoorFrame`) (`KismetMathLibrary.RLerp` (struct) (struct :`Yaw` -90.0) _doorrotation) false false)
          (if (`self.DoorOpen`)
            ;[1 1 1] 닫기를 생성하고 열기를 지움 DoorOpen = True
            (`|ExecutionSequence`
              (:`then_0`
                (`UserWidget.AddToViewport` _interactdoorclose 0))
              (:`then_1`
                (`Widget.RemoveFromParent` _interactdooropen)))
            (else
              ;[1 1 1] 열기를 생성하고 닫기를 지움 DoorOpen = False
              (`|ExecutionSequence`
                (:`then_0`
                  (`UserWidget.AddToViewport` _interactdooropen 0))
                (:`then_1`
                  (`Widget.RemoveFromParent` _interactdoorclose))))))))
    (:`B`
      (set `self.DoorOpen` false)
      (goto _label :!via `Reverse`))))

(event `self.ReceiveBeginPlay`
  (`|ExecutionSequence`
    (:`then_0`
      (bind _returnvalue (`|CreateWidget` "/Game/HouseOfChangwon/Blueprints/UI_CloseMessage.UI_CloseMessage_C"))
      (set `self.InteractDoorClose` _returnvalue))
    (:`then_1`
      (bind _returnvalue_2 (`|CreateWidget` "/Game/HouseOfChangwon/Blueprints/UI_OpenMessage.UI_OpenMessage_C"))
      (set `self.InteractDoorOpen` _returnvalue_2))))

(event `self.OverlapBox.OnComponentBeginOverlap`
  (params (OverlappedComponent :type "PrimitiveComponent Object Reference") (OtherActor :type "Actor Object Reference") (OtherComp :type "PrimitiveComponent Object Reference") (OtherBodyIndex :type Integer) (bFromSweep :type Boolean) (SweepResult :type "HitResult Structure (by ref)"))
  (if (== OtherActor (`GameplayStatics.GetPlayerCharacter` 0))
    (if (`self.DoorOpen`)
      (`UserWidget.AddToViewport` (`self.InteractDoorClose`) 0)
      (else
        (`UserWidget.AddToViewport` (`self.InteractDoorOpen`) 0)))))

(event `self.OverlapBox.OnComponentEndOverlap`
  (params (OverlappedComponent :type "PrimitiveComponent Object Reference") (OtherActor :type "Actor Object Reference") (OtherComp :type "PrimitiveComponent Object Reference") (OtherBodyIndex :type Integer))
  (if (== (`GameplayStatics.GetPlayerCharacter` 0) OtherActor)
    (if (`self.DoorOpen`)
      (`Widget.RemoveFromParent` (`self.InteractDoorClose`))
      (else
        (`Widget.RemoveFromParent` (`self.InteractDoorOpen`))))))

(fn `UserConstructionScript`)