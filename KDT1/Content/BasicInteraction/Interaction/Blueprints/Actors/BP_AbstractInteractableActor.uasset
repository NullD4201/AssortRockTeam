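; Base interactable actor that shows a prompt widget on focus and supports instant or hold-style timed interactions.
; A Radial flag selects either a radial prompt, filled through a material Alpha parameter, or a progress-bar prompt.
; Interaction events drive a timeline scaled to InteractionTimeS that updates the progress display and fires the PerformAction dispatcher on completion, or immediately when no time is set.
; Ending interaction stops the timeline, resets progress and refreshes the prompt text.
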(event `self.ReceiveBeginPlay`
  ;[1 1 1] Begin play
  (`self.F_UpdatePromptWidget`))

(event `self.IE_BeginInteraction`
  ;[1 1 1] Begin interaction
  (if (> (`self.InteractionTimeS`) 0.0)
    (`TimelineComponent.SetPlayRate` (`self.InteractionProgress`) (/ 1.0 (`self.InteractionTimeS`)))
    (bind (_direction _percent) (`Timeline|InteractionProgress` :!via `PlayFromStart`)
      (:`Update`
        (if (`self.Radial`)
          (bind _returnvalue (`Border.GetDynamicMaterial` (`/Game/BasicInteraction/Interaction/Blueprints/Widgets/WBP_InteractionPromptRadial.Progress_Circle` (`self.PromptWidgetRadialRef`))))
          (`MaterialInstanceDynamic.SetScalarParameterValue` _returnvalue "Alpha" _percent)
          (else
            (`ProgressBar.SetPercent` (`/Game/BasicInteraction/Interaction/Blueprints/Widgets/WBP_InteractionPrompt.ProgressBar` (`self.PromptWidgetRef`)) _percent))))
      (:`Finished`
        (`self.ED_PerformAction` self)
        (`self.IE_EndInteraction`)))
    (else
      (`self.ED_PerformAction` self)
      (`self.F_UpdatePromptWidget`))))

(event `self.IE_OnFocus`
  (params (Char :type "Character Object Reference"))
  ;[1 1 1] Show / hide prompt widget on focus
  (if (`self.Radial`)
    (`SceneComponent.SetVisibility` (`self.PromptWidgetRadial`) true false)
    (else
      (`SceneComponent.SetVisibility` (`self.PromptWidget`) true false))))

(event `self.IE_OnFocusLost`
  (params (Char :type "Character Object Reference"))
  ;[1 1 1] Show / hide prompt widget on focus
  (`SceneComponent.SetVisibility` (`self.PromptWidgetRadial`) false false)
  (`SceneComponent.SetVisibility` (`self.PromptWidget`) false false))

(event `self.IE_EndInteraction`
  (bind _promptwidgetref (`self.PromptWidgetRef`))
  ;[1 1 1] End interaction - hide loader, update prompt
  (`TimelineComponent.Stop` (`self.InteractionProgress`))
  (if (`self.Radial`)
    (bind _returnvalue (`Border.GetDynamicMaterial` (`/Game/BasicInteraction/Interaction/Blueprints/Widgets/WBP_InteractionPromptRadial.Progress_Circle` (`self.PromptWidgetRadialRef`))))
    (`MaterialInstanceDynamic.SetScalarParameterValue` _returnvalue "Alpha" 0.0)
    (`self.F_UpdatePromptWidget`)
    (else
      (`/Engine/EditorBlueprintResources/StandardMacros.IsValid` _promptwidgetref
        (:`Is Valid`
          (`ProgressBar.SetPercent` (`/Game/BasicInteraction/Interaction/Blueprints/Widgets/WBP_InteractionPrompt.ProgressBar` _promptwidgetref) 0.0)
          (`self.F_UpdatePromptWidget`))))))

(fn `F_UpdatePromptWidget`
  (bind _promptwidgetradial (`self.PromptWidgetRadial`))
  (if (`self.Radial`)
    (`/Engine/EditorBlueprintResources/StandardMacros.IsValid` _promptwidgetradial
      (:`Is Valid`
        (bind _aswbp_interaction_prompt_radial (cast `/Game/BasicInteraction/Interaction/Blueprints/Widgets/WBP_InteractionPromptRadial` (`WidgetComponent.GetWidget` _promptwidgetradial)))
        (bind _output_get (set `self.PromptWidgetRadialRef` _aswbp_interaction_prompt_radial))
        (`/Game/BasicInteraction/Interaction/Blueprints/Widgets/WBP_InteractionPromptRadial.E_UpdatePrompt` _output_get (`self.PromptText`))))
    (else
      (`/Engine/EditorBlueprintResources/StandardMacros.IsValid` (`self.PromptWidget`)
        (:`Is Valid`
          (bind _aswbp_interaction_prompt (cast `/Game/BasicInteraction/Interaction/Blueprints/Widgets/WBP_InteractionPrompt` (`WidgetComponent.GetWidget` (`self.PromptWidget`))))
          (bind _output_get_2 (set `self.PromptWidgetRef` _aswbp_interaction_prompt))
          (`/Game/BasicInteraction/Interaction/Blueprints/Widgets/WBP_InteractionPrompt.E_UpdateWidget` _output_get_2 (`self.ItemName`) (`self.PromptText`) (`self.HideName`)))))))

(fn `UserConstructionScript`)