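; BP_Door is an interactable door that swings open and closed when the player performs its action.
; The interaction event calls MC_ToggleDoor, which sets IsOpened from whether the door's yaw is zero, then plays or reverses a Timeline driving that yaw.
; F_UpdatePromptWidget overrides the parent function to set the prompt to "Open" or "Close" from IsOpened before calling the parent.
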(event `/Game/BasicInteraction/Interaction/Blueprints/Interfaces/BPI_Interaction.IE_PerformAction`
  (params (Char :type "Character Object Reference"))
  (`self.MC_ToggleDoor`))

(event `MC_ToggleDoor`
  (bind (_relativerotation_roll _relativerotation_pitch _relativerotation_yaw) (`KismetMathLibrary.BreakRotator` (`SceneComponent.RelativeRotation` (`self.Door`))))
  (bind _returnvalue (== _relativerotation_yaw 0.0))
  (set `self.IsOpened` _returnvalue)
  (if _returnvalue
    (bind (_direction _rotation) (`Timeline|Timeline_1` :!label _label)
      (:`Update`
        (`SceneComponent.K2_SetRelativeRotation` (`self.Door`) (`KismetMathLibrary.MakeRotator` 0.0 0.0 _rotation) false false)))
    (else
      (goto _label :!via `Reverse`))))

(fn `F_UpdatePromptWidget`
  (`|ExecutionSequence`
    (:`then_0`
      (if (`self.IsOpened`)
        (set `self.PromptText` "Close")
        (else
          (set `self.PromptText` "Open"))))
    (:`then_1`
      (`parent.F_UpdatePromptWidget`))))

(fn `UserConstructionScript`
  (`parent.UserConstructionScript`))