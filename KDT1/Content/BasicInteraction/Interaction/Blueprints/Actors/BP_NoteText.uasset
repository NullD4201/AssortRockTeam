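; BP_NoteText is an interactable note actor that shows a text note on screen when its interaction action runs.
; IEPerformAction calls CL_ShowNote, which removes any top-level WBP_TextNote widgets, then creates one from NoteSettings and adds it to the viewport.
; IF_CanInteract looks up open note widgets but leaves the result unused, returning no computed value.
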(event `/Game/BasicInteraction/Interaction/Blueprints/Interfaces/BPI_Interaction.IE_PerformAction`
  (params (Char :type "Character Object Reference"))
  (`self.CL_ShowNote`))

(event `CL_ShowNote`
  (`|ExecutionSequence`
    (:`then_0`
      (bind _foundwidgets (`WidgetBlueprintLibrary.GetAllWidgetsOfClass` "/Game/BasicInteraction/Interaction/Blueprints/Widgets/WBP_TextNote.WBP_TextNote_C"))
      (for _array_element _foundwidgets
        (`Widget.RemoveFromParent` _array_element)))
    (:`then_1`
      (bind _returnvalue (`|CreateWidget` "/Game/BasicInteraction/Interaction/Blueprints/Widgets/WBP_TextNote.WBP_TextNote_C" null (`self.NoteSettings`)))
      (`UserWidget.AddToViewport` _returnvalue 0))))

(fn `IF_CanInteract`
  (bind _foundwidgets (`WidgetBlueprintLibrary.GetAllWidgetsOfClass` "/Game/BasicInteraction/Interaction/Blueprints/Widgets/WBP_TextNote.WBP_TextNote_C"))
  (return))

(fn `UserConstructionScript`)