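; BP_NoteAudio is an interactable note actor that shows an audio note widget on screen when its perform-action event fires.
; The action calls the CL_ShowNote event, which first removes every top-level WBP_AudioNote already displayed.
; It then creates a new WBP_AudioNote from the actor's NoteSettings and adds it to the viewport, so only one audio note shows at a time.
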(event `/Game/BasicInteraction/Interaction/Blueprints/Interfaces/BPI_Interaction.IE_PerformAction`
  (params (Char :type "Character Object Reference"))
  (`self.CL_ShowNote`))

(event `CL_ShowNote`
  (`|ExecutionSequence`
    (:`then_0`
      (bind _foundwidgets (`WidgetBlueprintLibrary.GetAllWidgetsOfClass` "/Game/BasicInteraction/Interaction/Blueprints/Widgets/WBP_AudioNote.WBP_AudioNote_C"))
      (for _array_element _foundwidgets
        (`Widget.RemoveFromParent` _array_element)))
    (:`then_1`
      (bind _returnvalue (`|CreateWidget` "/Game/BasicInteraction/Interaction/Blueprints/Widgets/WBP_AudioNote.WBP_AudioNote_C" null (`self.NoteSettings`)))
      (`UserWidget.AddToViewport` _returnvalue 0))))

(fn `UserConstructionScript`
  (`parent.UserConstructionScript`))