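; Character component that lets the player focus and interact with world actors through InteractionInterface.
; Each tick it line-traces from the player camera, sending focus and focus-lost messages and caching the looked-at actor.
; Begin and end events message that actor, binding interactable actors' perform-action dispatcher to SRV_Interact, which assigns character ownership before performing the action.
; A helper event also removes all text and audio note widgets.
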(event `self.ReceiveBeginPlay`
  ;[1 1 1] Get owner character ref
  (bind _ascharacter (cast `Character` (`self.GetOwner`)))
  (set `self.CharacterRef` _ascharacter))

(event `SRV_Interact`
  (params (Actor :type "Actor Object Reference"))
  ;[0 0.6251 1] Begin interaction
  (`Actor.SetOwner` Actor (`self.CharacterRef`))
  (message `/Game/BasicInteraction/Interaction/Blueprints/Interfaces/BPI_Interaction.IE_PerformAction` Actor (`self.CharacterRef`)))

(event `E_BeginInteraction`
  (bind _activeactor (`self.F_GetActiveActor`))
  ;[0 0.6251 1] Begin interaction
  (`|ExecutionSequence`
    (:`then_0`
      (`/Engine/EditorBlueprintResources/StandardMacros.IsValid` _activeactor
        (:`Is Valid`
          (bind _asbp_abstract_interactable_actor (cast `/Game/BasicInteraction/Interaction/Blueprints/Actors/BP_AbstractInteractableActor` _activeactor))
          (add `/Game/BasicInteraction/Interaction/Blueprints/Actors/BP_AbstractInteractableActor.ED_PerformAction` _asbp_abstract_interactable_actor (delegate `SRV_Interact`)))))
    (:`then_1`
      (message `/Game/BasicInteraction/Interaction/Blueprints/Interfaces/BPI_Interaction.IE_BeginInteraction` _activeactor))))

(event `self.ReceiveTick`
  (params (DeltaSeconds :type "Float (single-precision)"))
  (bind (_start _end) (`self.F_GetTrace`))
  ;[1 1 1] Tick - line trace, search ray
  (`self.F_SearchRay` _start _end))

(event `E_EndInteraction`
  (bind _activeactor (`self.F_GetActiveActor`))
  ;[0 0.6251 1] End interaction
  (`/Engine/EditorBlueprintResources/StandardMacros.IsValid` _activeactor
    (:`Is Valid`
      (message `/Game/BasicInteraction/Interaction/Blueprints/Interfaces/BPI_Interaction.IE_EndInteraction` _activeactor))))

(event `E_RemoveAllNotes`
  ;[1 1 1] Remove note widgets - better use it in player controller
  (`|ExecutionSequence`
    (:`then_0`
      (bind _foundwidgets (`WidgetBlueprintLibrary.GetAllWidgetsOfClass` "/Game/BasicInteraction/Interaction/Blueprints/Widgets/WBP_TextNote.WBP_TextNote_C"))
      (for _array_element _foundwidgets
        (`Widget.RemoveFromParent` _array_element)))
    (:`then_1`
      (bind _foundwidgets_2 (`WidgetBlueprintLibrary.GetAllWidgetsOfClass` "/Game/BasicInteraction/Interaction/Blueprints/Widgets/WBP_AudioNote.WBP_AudioNote_C"))
      (for _array_element_2 _foundwidgets_2
        (`Widget.RemoveFromParent` _array_element_2)))))

(event `SRV_SetInteractableActorOwner`
  (params (Actor :type "Actor Object Reference"))
  ;[0 0.6251 1] End interaction
  (`Actor.SetOwner` Actor (`self.CharacterRef`))
  (message `/Game/BasicInteraction/Interaction/Blueprints/Interfaces/BPI_Interaction.IE_PerformAction` Actor (`self.CharacterRef`)))

(fn `F_GetActiveActor`
  (returns (ActiveActor :type "Actor Object Reference"))
  (return (`self.ActorYouAreLookingAt`)))

(fn `F_GetTrace`
  (returns (Start :type "Vector Structure") (End :type "Vector Structure"))
  (bind _returnvalue (`GameplayStatics.GetPlayerCameraManager` 0))
  (bind _returnvalue_2 (`Actor.GetActorForwardVector` _returnvalue))
  (bind _returnvalue_3 (`Actor.K2_GetActorLocation` _returnvalue))
  (return (+ _returnvalue_3 (* _returnvalue_2 (`self.TraceForwardCameraOffset`))) (+ (* _returnvalue_2 (`self.Tracelength`)) _returnvalue_3)))

(fn `F_SearchRay`
  (params (Start :type "Vector Structure") (End :type "Vector Structure"))
  (bind _actoryouarelookingat (`self.ActorYouAreLookingAt`))
  (bind (_outhit _returnvalue) (`KismetSystemLibrary.LineTraceSingle` Start End "TraceTypeQuery1" false (`|MakeArray` (`self.GetOwner`)) (`self.DrawDebugType`)))
  (if _returnvalue
    (bind (_bblockinghit _binitialoverlap _time _distance _location _impactpoint _normal _impactnormal _physmat _hitactor) (`GameplayStatics.BreakHitResult` _outhit))
    (if (`KismetSystemLibrary.DoesImplementInterface` _hitactor (`self.InteractionInterface`))
      ;[1 1 1] On focus
      (`/Engine/EditorBlueprintResources/StandardMacros.IsValid` (`self.ActorYouAreLookingAt`)
        (:`Is Not Valid`
          (bind _output_get (set `self.ActorYouAreLookingAt` _hitactor))
          (message `/Game/BasicInteraction/Interaction/Blueprints/Interfaces/BPI_Interaction.IE_OnFocus` _output_get (`self.CharacterRef`))))
      (else
        ;[1 1 1] Lost focus
        (`/Engine/EditorBlueprintResources/StandardMacros.IsValid` _actoryouarelookingat :!label _label
          (:`Is Valid`
            (message `/Game/BasicInteraction/Interaction/Blueprints/Interfaces/BPI_Interaction.IE_OnFocusLost` _actoryouarelookingat (`self.CharacterRef`))
            (message `/Game/BasicInteraction/Interaction/Blueprints/Interfaces/BPI_Interaction.IE_EndInteraction` (`self.ActorYouAreLookingAt`))
            (set `self.ActorYouAreLookingAt` null)))))
    (else
      (goto _label))))